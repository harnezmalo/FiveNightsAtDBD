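; Door actor that swings open away from either of two trigger boxes, with push-door sounds.
; BoxYMinus and BoxYAdd begin overlaps drive timelines that lerp Door yaw 90 degrees in opposite directions when Open is false.
; End overlaps hold reverse timelines with a closing sound on finish, but their checks require Open to be both true and false, so as written they never run.
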(event `self.BoxYMinus.OnComponentBeginOverlap`
  (params (OverlappedComponent :type "PrimitiveComponent Object Reference") (OtherActor :type "Actor Object Reference") (OtherComp :type "PrimitiveComponent Object Reference") (OtherBodyIndex :type Integer) (bFromSweep :type Boolean) (SweepResult :type "HitResult Structure (by ref)"))
  (if (and (== (`self.Open+`) false) (== (`self.Open-`) false))
    (`GameplayStatics.PlaySound2D` "/Game/Sounds/Sounds/SFX_PUSH_DOOR_OPEN.SFX_PUSH_DOOR_OPEN" 1.0 1.0 0.0 null null false)
    (bind (_direction _newtrack_0) (`Timeline|Timeline` :!via `PlayFromStart`)
      (:`Update`
        (`SceneComponent.K2_SetRelativeRotation` (`self.Door`) (`KismetMathLibrary.MakeRotator` 0.0 0.0 (`KismetMathLibrary.Lerp` 0.0 -90.0 _newtrack_0)) false false)
        (set `self.Open-` true)))))

(event `self.BoxYMinus.OnComponentEndOverlap`
  (params (OverlappedComponent :type "PrimitiveComponent Object Reference") (OtherActor :type "Actor Object Reference") (OtherComp :type "PrimitiveComponent Object Reference") (OtherBodyIndex :type Integer))
  (if (and (== (`self.Open+`) false) (== (`self.Open-`) true))
    (bind (_direction _newtrack_0) (`Timeline|Timeline_0` :!via `PlayFromStart`)
      (:`Update`
        (`SceneComponent.K2_SetRelativeRotation` (`self.Door`) (`KismetMathLibrary.MakeRotator` 0.0 0.0 (`KismetMathLibrary.Lerp` -90.0 0.0 _newtrack_0)) false false)
        (set `self.Open-` false))
      (:`Finished`
        (`GameplayStatics.PlaySound2D` "/Game/Sounds/Sounds/SFX_PUSH_DOOR_CLOSE.SFX_PUSH_DOOR_CLOSE" 1.0 1.0 0.0 null null false)))))

(event `self.BoxYAdd.OnComponentBeginOverlap`
  (params (OverlappedComponent :type "PrimitiveComponent Object Reference") (OtherActor :type "Actor Object Reference") (OtherComp :type "PrimitiveComponent Object Reference") (OtherBodyIndex :type Integer) (bFromSweep :type Boolean) (SweepResult :type "HitResult Structure (by ref)"))
  (if (and (== (`self.Open+`) false) (== (`self.Open-`) false))
    (`GameplayStatics.PlaySound2D` "/Game/Sounds/Sounds/SFX_PUSH_DOOR_OPEN.SFX_PUSH_DOOR_OPEN" 1.0 1.0 0.0 null null false)
    (bind (_direction _newtrack_0) (`Timeline|Timeline_1`)
      (:`Update`
        (`SceneComponent.K2_SetRelativeRotation` (`self.Door`) (`KismetMathLibrary.MakeRotator` 0.0 0.0 (`KismetMathLibrary.Lerp` 0.0 90.0 _newtrack_0)) false false)
        (set `self.Open+` true)))))

(event `self.BoxYAdd.OnComponentEndOverlap`
  (params (OverlappedComponent :type "PrimitiveComponent Object Reference") (OtherActor :type "Actor Object Reference") (OtherComp :type "PrimitiveComponent Object Reference") (OtherBodyIndex :type Integer))
  (if (and (== (`self.Open+`) true) (== (`self.Open-`) false))
    (bind (_direction _newtrack_0) (`Timeline|Timeline_2` :!via `PlayFromStart`)
      (:`Update`
        (`SceneComponent.K2_SetRelativeRotation` (`self.Door`) (`KismetMathLibrary.MakeRotator` 0.0 0.0 (`KismetMathLibrary.Lerp` 90.0 0.0 _newtrack_0)) false false)
        (set `self.Open+` false))
      (:`Finished`
        (`GameplayStatics.PlaySound2D` "/Game/Sounds/Sounds/SFX_PUSH_DOOR_CLOSE.SFX_PUSH_DOOR_CLOSE" 1.0 1.0 0.0 null null false)))))

(fn `UserConstructionScript`)