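; BP_PutDown is an interactible ingredient drop-off trigger that gates the player's progress.
; When BP_ThirdPersonCharacter overlaps its Box, it checks that the character's Ingrédients contain every entry in IngrédientsNécessaires.
; On success, the Fin flag selects between moving the player to the first actor tagged "Spawn2" and opening LevelDeFin, with a give-ingredient sound either way.
; The character's ingredient list is only read, never modified.
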(event `self.Box.OnComponentBeginOverlap`
  (params (OverlappedComponent :type "PrimitiveComponent Object Reference") (OtherActor :type "Actor Object Reference") (OtherComp :type "PrimitiveComponent Object Reference") (OtherBodyIndex :type Integer) (bFromSweep :type Boolean) (SweepResult :type "HitResult Structure (by ref)"))
  (bind _asbp_third_person_character (cast `/Game/ThirdPerson/Blueprints/BP_ThirdPersonCharacter` OtherActor))
  (set `self.Good` true)
  (for _array_element (`self.IngrédientsNécessaires`)
    (if (not (`KismetArrayLibrary.Array_Contains` (`/Game/ThirdPerson/Blueprints/BP_ThirdPersonCharacter.Ingrédients` _asbp_third_person_character) _array_element))
      (set `self.Good` false)))
  (if (and (`self.Good`) (== (`self.Fin`) false))
    (bind _outactors (`GameplayStatics.GetAllActorsWithTag` "Spawn2"))
    (`self.K2_SetActorLocation` _asbp_third_person_character (`self.K2_GetActorLocation` (`|GetArrayItem` _outactors)) false false)
    (`GameplayStatics.PlaySound2D` "/Game/Sounds/Sounds/SFX_GIVE_INGREDIENT.SFX_GIVE_INGREDIENT" 1.0 1.0 0.0 null null :!label _label)
    (elif (and (`self.Good`) (`self.Fin`))
      (`GameplayStatics.OpenLevel` (`self.LevelDeFin`))
      (goto _label))))

(fn `UserConstructionScript`)