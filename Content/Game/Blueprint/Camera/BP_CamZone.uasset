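; Camera trigger zone that switches the player's view to its linked BP_Cam when the third-person character enters its box.
; At BeginPlay it finds the camera with a matching zone index, then on overlap sets it as the character's current camera and view target.
; Safe zones also restart BP_AudioComp's random ambience on overlap begin and end.
; NouvelIndice assigns a new index above the highest found among existing zones.
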(event `self.ReceiveBeginPlay`
  (bind _outactors (`GameplayStatics.GetAllActorsOfClass` "/Game/Game/Blueprint/Camera/BP_Cam.BP_Cam_C"))
  (for _array_element _outactors
    (if (== (`/Game/Game/Blueprint/Camera/BP_Cam.IndiceZoneLiée` _array_element) (`self.IndiceZone`))
      (set `self.CameraLiee` _array_element))))

(event `self.Box.OnComponentBeginOverlap`
  (params (OverlappedComponent :type "PrimitiveComponent Object Reference") (OtherActor :type "Actor Object Reference") (OtherComp :type "PrimitiveComponent Object Reference") (OtherBodyIndex :type Integer) (bFromSweep :type Boolean) (SweepResult :type "HitResult Structure (by ref)"))
  (bind _cameraliee (`self.CameraLiee`))
  (bind _asbp_third_person_character (cast `/Game/ThirdPerson/Blueprints/BP_ThirdPersonCharacter` OtherActor))
  (`|ExecutionSequence`
    (:`then_0`
      (set `/Game/ThirdPerson/Blueprints/BP_ThirdPersonCharacter.CurrentCamera` _cameraliee _asbp_third_person_character)
      (`PlayerController.SetViewTargetWithBlend` (`GameplayStatics.GetPlayerController` 0) _cameraliee 0.0 "VTBlend_Linear" 0.0 false))
    (:`then_1`
      (if (`self.SafeZone`)
        (bind _returnvalue (`GameplayStatics.GetActorOfClass` "/Game/Sounds/NewFolder/BP_AudioComp.BP_AudioComp_C"))
        (`AudioComponent.Stop` (`/Game/Sounds/NewFolder/BP_AudioComp.Audio` _returnvalue))
        (`/Game/Sounds/NewFolder/BP_AudioComp.RandomAmb` _returnvalue)))))

(event `self.Box.OnComponentEndOverlap`
  (params (OverlappedComponent :type "PrimitiveComponent Object Reference") (OtherActor :type "Actor Object Reference") (OtherComp :type "PrimitiveComponent Object Reference") (OtherBodyIndex :type Integer))
  (if (`self.SafeZone`)
    (bind _returnvalue (`GameplayStatics.GetActorOfClass` "/Game/Sounds/NewFolder/BP_AudioComp.BP_AudioComp_C"))
    (`AudioComponent.Stop` (`/Game/Sounds/NewFolder/BP_AudioComp.Audio` _returnvalue))
    (`/Game/Sounds/NewFolder/BP_AudioComp.RandomAmb` _returnvalue)))

(fn `NouvelIndice`
  (locals (IndiceTemporaire :type Integer))
  (bind _outactors (`GameplayStatics.GetAllActorsOfClass` "BP_CamZone_C"))
  (for _array_element _outactors
    (bind _indicezone (`/Game/Game/Blueprint/Camera/BP_CamZone.IndiceZone` _array_element))
    (if (< (`local.IndiceTemporaire`) _indicezone)
      (set `local.IndiceTemporaire` _indicezone)))
  (set `self.IndiceZone` (+ (`local.IndiceTemporaire`) 1)))

(fn `UserConstructionScript`)