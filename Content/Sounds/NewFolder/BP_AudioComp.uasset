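; BP_AudioComp is an unfinished ambient sound Blueprint, apparently meant to play random backstore ambiences.
; BeginPlay fills a list with three 3D backstore sounds and caches the third-person player and all BP_CamZone actors.
; Play and RandomAmb are stubs with no effect.
; The disconnected playback logic would replace a stopped ambience with a random pick, though its random index never reaches the third sound.
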(event `self.ReceiveBeginPlay`
  (bind _sonsamb (`self.SonsAmb`))
  (`KismetArrayLibrary.Array_Add` _sonsamb "/Game/Sounds/Sounds/AMB/AMB_3D_BACKSTORE_01.AMB_3D_BACKSTORE_01")
  (`KismetArrayLibrary.Array_Add` _sonsamb "/Game/Sounds/Sounds/AMB/AMB_3D_BACKSTORE_02.AMB_3D_BACKSTORE_02")
  (`KismetArrayLibrary.Array_Add` _sonsamb "/Game/Sounds/Sounds/AMB/AMB_3D_BACKSTORE_03.AMB_3D_BACKSTORE_03")
  (bind _returnvalue (`GameplayStatics.GetActorOfClass` "/Game/ThirdPerson/Blueprints/BP_ThirdPersonCharacter.BP_ThirdPersonCharacter_C"))
  (set `self.Player` _returnvalue)
  (bind _outactors (`GameplayStatics.GetAllActorsOfClass` "/Game/Game/Blueprint/Camera/BP_CamZone.BP_CamZone_C"))
  (set `self.CamZones` _outactors))

(event `Play`
  (if (`AudioComponent.IsPlaying` (`self.Audio`))
    _))

(event `RandomAmb`
  (for _array_element (`self.CamZones`)
    (if true
      _)))

(fn `UserConstructionScript`)